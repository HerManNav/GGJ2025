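; Game mode for the bubble game that runs the match-start countdown and starts the gameplay music.
; On BeginPlay, timed delays step the MainHUD match-state text through "Ready" and "GO!" before hiding it.
; It then flags the game as running and unblocks input on the controlled BP_Player.
; A Sequence node starts the looping music in 2D alongside the countdown, and Tick is empty.
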(event `self.ReceiveBeginPlay`
  (bind _returnvalue (`GameplayStatics.GetPlayerController` 0))
  (`|ExecutionSequence`
    (:`then_0`
      (bind _asmain_hud (cast `/Game/Blueprints/UI/MainHUD` (`PlayerController.GetHUD` _returnvalue)))
      (bind _ui_ref (`/Game/Blueprints/UI/MainHUD.UI_Ref` _asmain_hud))
      (`/Game/Blueprints/UI/WB_MainUI.UpdateMatchStateText` _ui_ref "Ready")
      (`KismetSystemLibrary.Delay` 1.0)
      (`/Game/Blueprints/UI/WB_MainUI.UpdateMatchStateText` _ui_ref "GO!")
      (`KismetSystemLibrary.Delay` 0.5)
      (`/Game/Blueprints/UI/WB_MainUI.ChangeMatchStateTextVisibility` _ui_ref false)
      (set `self.bGameRunning` true)
      (bind _asbp_player (cast `/Game/Blueprints/Characters/Player/BP_Player` (`Controller.K2_GetPawn` _returnvalue)))
      (set `/Game/Blueprints/Characters/Player/BP_Player.bInputBlocked` false _asbp_player))
    (:`then_1`
      (`GameplayStatics.PlaySound2D` "/Game/Audio/Music/music_gameplay_loop.music_gameplay_loop" 0.2 1.0 0.0 null null))))

(event `self.ReceiveTick`
  (params (DeltaSeconds :type "Float (single-precision)")))

(fn `UserConstructionScript`)