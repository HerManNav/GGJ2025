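; BP_PlayerGameMode is a game mode that applies startup settings and shows the player's HUD.
; On BeginPlay it calls the parent, caps the frame rate through a console command, then creates WBP_HUD and adds it to the viewport.
; SpawnPlayer is effectively empty: its nodes for spawning the default pawn at CheckPoint and possessing it are disconnected, so they never run.
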(event `self.ReceiveBeginPlay`
  (`parent.ReceiveBeginPlay`)
  (`|ExecutionSequence`
    (:`then_0`
      (`KismetSystemLibrary.ExecuteConsoleCommand` "t.maxfps 120" null))
    (:`then_1`
      (bind _returnvalue (`|CreateWidget` "/Game/Blueprints/Widgets/WBP_HUD.WBP_HUD_C"))
      (`UserWidget.AddToViewport` _returnvalue 0))))

(fn `SpawnPlayer`)

(fn `UserConstructionScript`)