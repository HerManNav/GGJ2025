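; Bubble blob actor that draws a chain of bubble atoms as a spline mesh body with start and end caps.
; New atoms add segments, and Tick refits caps and segments to the spline.
; Blob events play sounds on closing or sticking, and evaluation adds a valid or invalid mesh at each atom's spline point.
; On explosion, it hides validity meshes, caps and segments and spawns burst effects along the spline.
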(event `self.ReceiveBeginPlay`
  (add `self.OnBlobAtomCreated` (delegate `OnBlobAtomCreated_Event_0`))
  (add `self.OnBlobClosed` (delegate `OnBlobClosed_Event`))
  (add `self.OnBlobStuck` (delegate `OnBlobStuck_Event`))
  (add `self.OnBlobExplosion` (delegate `OnBlobExplosion_Event`))
  (add `self.OnBlobEvaluation` (delegate `OnBlobEvaluation_Event`)))

(event `OnBlobAtomCreated_Event_0` :!signature `self.OnBlobAtomCreated`
  (params (BubbleAtomLocation :type "Vector Structure (by ref)"))
  (`self.GenerateMeshComponents`)
  (`self.UpdateMeshComponents`))

(event `OnBlobClosed_Event`
  (`GameplayStatics.PlaySound2D` "/Game/Audio/SFX/BubblePopCue.BubblePopCue" 1.0 1.0 0.0 null null))

(event `OnBlobStuck_Event`
  (`GameplayStatics.PlaySound2D` "/Game/Audio/SFX/Drips/DripDrop.DripDrop" 1.0 1.0 0.0 null null))

(event `OnBlobExplosion_Event` :!signature `self.OnBlobExplosion`
  (params (BubbleAtoms :type "Array of BubbleAtom Structure (by ref)"))
  ; explosion event, blob will be destroyed immediately
  (`self.ExplodeBlobs`))

(event `OnBlobEvaluation_Event` :!signature `self.OnBlobEvaluation`
  (params (BubbleAtoms :type "Array of BubbleAtom Structure (by ref)"))
  (for (_array_element _array_index) BubbleAtoms
    ; Red or green effects showing state of atom
    (`self.ShowBlobValidity` _array_index (break `BubbleAtom` _array_element))))

(event `self.ReceiveTick`
  (params (DeltaSeconds :type "Float (single-precision)"))
  (`self.UpdateMeshComponents`))

(fn `ExplodeBlobs`
  (bind _startcap (`self.StartCap`))
  (bind _end_cap (`self.End Cap`))
  ; Hide invalid blobs
  (for _array_element (`self.MC_ValidityBlob`)
    (`SceneComponent.SetVisibility` _array_element false false)
    ; Pop Spline Start cap
    (`SceneComponent.SetVisibility` _startcap false false)
    (`NiagaraFunctionLibrary.SpawnSystemAttached` (`self.BurstEmitter`) _startcap "None" (0.0 0.0 0.0) (struct) "KeepRelativeOffset" true)
    ; Pop Spline Middle Sections
    (for (_array_element_2 _array_index) (`self.SMC_BlobSegment`)
      (`SceneComponent.SetVisibility` _array_element_2 false false)
      (`NiagaraFunctionLibrary.SpawnSystemAtLocation` (`self.BurstEmitter`) (.location (`SplineComponent.GetTransformAtSplinePoint` (`self.SplineComponent`) (+ _array_index 1) "World" false)) (.rotation (`SplineComponent.GetTransformAtSplinePoint` (`self.SplineComponent`) (+ _array_index 1) "World" false)) (.scale (`SplineComponent.GetTransformAtSplinePoint` (`self.SplineComponent`) (+ _array_index 1) "World" false)))
      ; Pop Spline End cap
      (`SceneComponent.SetVisibility` _end_cap false false)
      (`NiagaraFunctionLibrary.SpawnSystemAttached` (`self.BurstEmitter`) _end_cap "None" (0.0 0.0 0.0) (struct) "KeepRelativeOffset" true))))

(fn `GenerateMeshComponents`
  (bind _splinecomponent (`self.SplineComponent`))
  (bind _splinecomponent_2 (`self.SplineComponent`))
  ; Add Spline Middle Sections
  (for _index (range (`KismetArrayLibrary.Array_Length` (`self.SMC_BlobSegment`)) (+ (- (`SplineComponent.GetNumberOfSplinePoints` (`self.SplineComponent`)) 2) 1))
    (bind _returnvalue (`AddComponent|NODE_AddSplineMeshComponent-7`))
    (`KismetArrayLibrary.Array_Add` (`self.SMC_BlobSegment`) _returnvalue)
    (`StaticMeshComponent.SetStaticMesh` _returnvalue (`self.BlobMiddle`))
    (`SplineMeshComponent.SetForwardAxis` _returnvalue (`self.In Forward Axis`) true)
    (bind _returnvalue_2 (+ _index 1))
    (`SplineMeshComponent.SetStartAndEnd` _returnvalue (`SplineComponent.GetLocationAtSplinePoint` _splinecomponent_2 _index "Local") (`SplineComponent.GetTangentAtSplinePoint` _splinecomponent_2 _index "Local") (`SplineComponent.GetLocationAtSplinePoint` _splinecomponent _returnvalue_2 "Local") (`SplineComponent.GetTangentAtSplinePoint` _splinecomponent _returnvalue_2 "Local") true)))

(fn `ShowBlobValidity`
  (params (BlobIndex :type Integer) (BlobValid :type Boolean))
  (bind _returnvalue (`AddComponent|NODE_AddStaticMeshComponent-14` :`RelativeTransform` (`SplineComponent.GetTransformAtSplinePoint` (`self.SplineComponent`) BlobIndex "Local" false)))
  (if BlobValid
    (`StaticMeshComponent.SetStaticMesh` _returnvalue (`self.ValidBlob`))
    (else
      (`StaticMeshComponent.SetStaticMesh` _returnvalue (`self.InvalidBlob`))))
  (`KismetArrayLibrary.Array_Add` (`self.MC_ValidityBlob`) _returnvalue))

(fn `UpdateMeshComponents`
  (bind _splinecomponent (`self.SplineComponent`))
  (bind _splinecomponent_2 (`self.SplineComponent`))
  (bind _splinecomponent_3 (`self.SplineComponent`))
  ; Add Spline Start cap
  (`SceneComponent.K2_SetRelativeTransform` (`self.StartCap`) (`SplineComponent.GetTransformAtSplinePoint` (`self.SplineComponent`) 0 "Local" false) false false)
  (`SceneComponent.K2_AddRelativeRotation` (`self.StartCap`) (struct :`Pitch` 90.0) false false)
  ; Add Spline End cap
  (`SceneComponent.K2_SetRelativeTransform` (`self.End Cap`) (`SplineComponent.GetTransformAtSplinePoint` _splinecomponent_3 (`SplineComponent.GetNumberOfSplinePoints` _splinecomponent_3) "Local" false) false false)
  (`SceneComponent.K2_AddRelativeRotation` (`self.End Cap`) (struct :`Pitch` 270.0) false false)
  ; Add Spline Middle Sections
  (for (_array_element _array_index) (`self.SMC_BlobSegment`)
    (bind _returnvalue (+ _array_index 1))
    (`SplineMeshComponent.SetStartAndEnd` _array_element (`SplineComponent.GetLocationAtSplinePoint` _splinecomponent_2 _array_index "Local") (`SplineComponent.GetTangentAtSplinePoint` _splinecomponent_2 _array_index "Local") (`SplineComponent.GetLocationAtSplinePoint` _splinecomponent _returnvalue "Local") (`SplineComponent.GetTangentAtSplinePoint` _splinecomponent _returnvalue "Local") true)))

(fn `UserConstructionScript`
  (`self.GenerateMeshComponents`)
  (`self.UpdateMeshComponents`))